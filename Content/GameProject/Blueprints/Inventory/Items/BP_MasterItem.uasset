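; BP_MasterItem is a world item actor that characters can pick up, building its item object and amount from its base data in the construction script.
; Interact first tries the character's equipment, then falls back to an available inventory found through that equipment.
; RefreshItem stores what remains and destroys the actor once the amount drops below one.
; GroundInteraction passes the item and actor to the inventory's ground items.
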(event EventGroundInteraction
  (params (Char :type Third%20Person%20Character%20Object%20Reference))
  (Default|AddItemstotheGround (Variables|/Game/GameProject/Blueprints/ThirdPersonCharacter.ThirdPersonCharacter_C|GetInventory Char) (Variables|ItemPrivate|GetItem) self))

(event EventInteract
  (params (Char :type Third%20Person%20Character%20Object%20Reference))
  (bind _equipment (Variables|/Game/GameProject/Blueprints/ThirdPersonCharacter.ThirdPersonCharacter_C|GetEquipment Char))
  (bind _inventory (Variables|/Game/GameProject/Blueprints/ThirdPersonCharacter.ThirdPersonCharacter_C|GetInventory Char))
  (bind (_return _returnitem) (Default|TryAddItem _equipment (Variables|ItemPrivate|GetItem)))
  (if _return
    (Private|RefreshItem _returnitem)
    (Default|RefreshInventory _inventory)
    (else
      (bind (_return_2 _inventory_2) (Default|SearchforAvaliableInventory _equipment (Variables|ItemPrivate|GetItem)))
      (if _return_2
        (bind (_return_3 _restofitems) (Default|AddItemtoInventory _inventory _inventory_2 (Variables|ItemPrivate|GetItem)))
        (if _return_3
          (Private|RefreshItem _restofitems))))))

(fn ConstructionScript
  (bind _self self)
  (bind _basedata (Variables|Default|GetBaseData))
  (bind _returnvalue (Game|ConstructObjectfromClass _self "/Game/GameProject/Blueprints/Inventory/Items/BP_BaseItemObject.BP_BaseItemObject_C" (.name _basedata) (.description _basedata) (.icon _basedata) (Utilities|GetClass _self) (.equipmenttype _basedata) (.itemsize _basedata) (Variables|Default|GetMax%20Stack%20Size) (Variables|Default|GetSkeletal%20Mesh) (Variables|Default|GetStaticMeshObj)))
  (Variables|ItemPrivate|SetItem (Utilities|Struct|MakeItemStructure _returnvalue (Variables|Default|GetAmount))))

(fn RefreshItem
  (params (Item :type Item%20Structure%20Structure))
  (Variables|ItemPrivate|SetItem Item)
  (if (< (.amount (Variables|ItemPrivate|GetItem)) 1)
    (Actor|DestroyActor)))