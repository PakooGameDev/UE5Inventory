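; Inventory component that manages items in wearable storage items, a fixed-slot container and a list of nearby ground items.
; Adds stack by item class or fill empty slots, and changes to wearable storage also update its capacity.
; Dropped items respawn as physics actors, with uniforms, vests and backpacks keeping their contents, then a sphere trace rebuilds the ground list through interface messages.
; It also swaps equipment slots and toggles the inventory UI.
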(event EventBeginPlay
  (CallFunction|Initialize (Variables|Default|GetContainer%20Size)))

(fn AddItemtoInventory
  (params (TargetInventory :type Item%20Structure%20Structure) (Item :type Item%20Structure%20Structure))
  (bind _asbp_inventory_item (Utilities|Casting|CastToBP_InventoryItem (.item TargetInventory)))
  (bind (_array_element _array_index) (Utilities|Array|ForEachLoopwithBreak (Variables|/Game/GameProject/Blueprints/Inventory/Items/BP_InventoryItem.BP_InventoryItem_C|GetInventory _asbp_inventory_item) :!label _label)
    (:LoopBody
      (Utilities|IsValid? _array_element
        (:IsValid
          (LocalVariables|SetLocalIndex _array_index)
          (LocalVariables|SetLocalSlot _array_element)
          (if (and (Checks|SameItems? (LocalVariables|GetLocalSlot) Item) (Checks|IsStackAvaliable? (LocalVariables|GetLocalSlot)))
            (Utilities|Array|SetArrayElem (Variables|/Game/GameProject/Blueprints/Inventory/Items/BP_InventoryItem.BP_InventoryItem_C|GetInventory _asbp_inventory_item) (LocalVariables|GetLocalIndex) (Utilities|Struct|MakeItemStructure (.item (LocalVariables|GetLocalSlot)) (+ (.amount (LocalVariables|GetLocalSlot)) 1)))
            (UpdateCapacity|UpdateCapacityonAdd TargetInventory Item)
            (LocalVariables|SetSuccess true)
            (goto _label Break)
            (else
              (LocalVariables|SetSuccess false))))
        (:IsNotValid
          (LocalVariables|SetEmptySlotIndex _array_index)
          (LocalVariables|SetFoundEmptySlot true))))
    (:Completed
      (if (LocalVariables|GetSuccess)
        _
        (elif (LocalVariables|GetFoundEmptySlot)
          (Utilities|Array|SetArrayElem (Variables|/Game/GameProject/Blueprints/Inventory/Items/BP_InventoryItem.BP_InventoryItem_C|GetInventory _asbp_inventory_item) (LocalVariables|GetEmptySlotIndex) (Utilities|Struct|MakeItemStructure (.item Item) 1))
          (LocalVariables|SetSuccess true)
          (UpdateCapacity|UpdateCapacityonAdd TargetInventory Item)
          (else
            (return false Item))))
      (ConstructWidgets|RefreshInventory)
      (return true (Utilities|Struct|MakeItemStructure (.item Item) (- (.amount Item) 1))))))

(fn IsStackAvaliable?
  (params (Item :type Item%20Structure%20Structure))
  (bind (_item _amount) (Utilities|Struct|BreakItemStructure Item))
  (return (<= (+ _amount 1) (Variables|/Game/GameProject/Blueprints/Inventory/Items/BP_BaseItemObject.BP_BaseItemObject_C|GetMaxStackSize _item))))

(fn RemoveAmountfromInventory
  (params (Inventory :type Item%20Structure%20Structure) (ItemIndex :type Integer) (AmountToRemove :type Integer))
  (bind _asbp_inventory_item (Utilities|Casting|CastToBP_InventoryItem (.item Inventory)))
  (LocalVariables|SetInventoryItem (Utilities|Array|Get(acopy) (Variables|/Game/GameProject/Blueprints/Inventory/Items/BP_InventoryItem.BP_InventoryItem_C|GetInventory _asbp_inventory_item) ItemIndex))
  (LocalVariables|SetAmountInInventory (- (.amount (LocalVariables|GetInventoryItem)) AmountToRemove))
  (if (<= (LocalVariables|GetAmountInInventory) 0)
    (Utilities|Array|RemoveIndex (Variables|/Game/GameProject/Blueprints/Inventory/Items/BP_InventoryItem.BP_InventoryItem_C|GetInventory _asbp_inventory_item) ItemIndex)
    (UpdateCapacity|UpdateCapacityonRemove Inventory (LocalVariables|GetInventoryItem))
    (return (LocalVariables|GetInventoryItem))
    (else
      (Utilities|Array|SetArrayElem (Variables|/Game/GameProject/Blueprints/Inventory/Items/BP_InventoryItem.BP_InventoryItem_C|GetInventory _asbp_inventory_item) ItemIndex (Utilities|Struct|MakeItemStructure (.item (LocalVariables|GetInventoryItem)) (LocalVariables|GetAmountInInventory)))
      (UpdateCapacity|UpdateCapacityonRemove Inventory (LocalVariables|GetInventoryItem) (LocalVariables|GetAmountInInventory))
      (return (Utilities|Struct|MakeItemStructure (.item (LocalVariables|GetInventoryItem)) AmountToRemove)))))

(fn RefreshInventory
  (Default|CallRefreshDispatcher)
  (Development|PrintString "Hello"))

(fn ToggleInventory
  (params (Source :type Source%20Enum :default "NewEnumerator1") (BPContainer :type BP%20Container%20Object%20Reference))
  (bind _returnvalue (Game|GetPlayerController 0))
  (bind _returnvalue_2 (Game|GetPlayerController 0))
  (Variables|Default|GetUI_InventoryRef
    (:then
      (switch Utilities|FlowControl|Switch|SwitchonESlateVisibility (Widget|GetVisibility (Variables|Default|GetUI_InventoryRef))
        (:Visible
          (Widget|SetVisibility (Variables|Default|GetUI_InventoryRef) "Collapsed")
          (Variables|/Script/Engine.PlayerController|SetbShowMouseCursor _returnvalue false)
          (Input|SetInputModeGameOnly _returnvalue false)
          (Class|BIContextMenu|RemoveContextMenu(Message) (Variables|Default|GetUI_InventoryRef)))
        (:Collapsed
          (Variables|/Game/GameProject/Blueprints/Inventory/UI/UI_PlayerInfo.UI_PlayerInfo_C|SetBPContainer (Variables|Default|GetUI_InventoryRef) BPContainer)
          (Widget|SetVisibility (Variables|Default|GetUI_InventoryRef) "Visible")
          (Class|BIOpenInventory|OpenInventory(Message) :self (Variables|Default|GetUI_InventoryRef) :Source Source)
          (Default|CallRefreshDispatcher)
          (Variables|/Script/Engine.PlayerController|SetbShowMouseCursor _returnvalue_2 true :!label _label)
          (Input|SetInputModeGameandUI _returnvalue_2 (Variables|Default|GetUI_InventoryRef) "DoNotLock" true false))))
    (:else
      (bind _returnvalue_3 (UserInterface|CreateWidget "/Game/GameProject/Blueprints/Inventory/UI/UI_PlayerInfo.UI_PlayerInfo_C" 0 BPContainer))
      (bind _output_get (Variables|Default|SetUI_InventoryRef _returnvalue_3))
      (UserInterface|Viewport|AddtoViewport _output_get 0)
      (Class|BIOpenInventory|OpenInventory(Message) :self (Variables|Default|GetUI_InventoryRef) :Source Source)
      (Widget|SetVisibility (Variables|Default|GetUI_InventoryRef) "Visible")
      (goto _label))))

(fn SameItems?
  (params (LocalItem :type Item%20Structure%20Structure) (AddItem :type Item%20Structure%20Structure))
  (return (== (Variables|/Game/GameProject/Blueprints/Inventory/Items/BP_BaseItemObject.BP_BaseItemObject_C|GetItemClass (.Item (Utilities|Struct|BreakItemStructure LocalItem))) (Variables|/Game/GameProject/Blueprints/Inventory/Items/BP_BaseItemObject.BP_BaseItemObject_C|GetItemClass (.Item (Utilities|Struct|BreakItemStructure AddItem))))))

(fn UpdateCapacityonRemove
  (params (OldItem :type Item%20Structure%20Structure) (Item :type Item%20Structure%20Structure) (AmountToRemove :type Integer))
  (bind _asbp_inventory_item (Utilities|Casting|CastToBP_InventoryItem (.item OldItem)))
  (Variables|/Game/GameProject/Blueprints/Inventory/Items/BP_InventoryItem.BP_InventoryItem_C|SetCurrentCapacity _asbp_inventory_item (- (Variables|/Game/GameProject/Blueprints/Inventory/Items/BP_InventoryItem.BP_InventoryItem_C|GetCurrentCapacity _asbp_inventory_item) (* (Variables|/Game/GameProject/Blueprints/Inventory/Items/BP_BaseItemObject.BP_BaseItemObject_C|GetItemSize (.item Item)) (- (.amount Item) AmountToRemove)))))

(fn UpdateCapacityonAdd
  (params (OldItem :type Item%20Structure%20Structure) (Item :type Item%20Structure%20Structure))
  (bind _asbp_inventory_item (Utilities|Casting|CastToBP_InventoryItem (.item OldItem)))
  (Variables|/Game/GameProject/Blueprints/Inventory/Items/BP_InventoryItem.BP_InventoryItem_C|SetCurrentCapacity _asbp_inventory_item (+ (Variables|/Game/GameProject/Blueprints/Inventory/Items/BP_InventoryItem.BP_InventoryItem_C|GetCurrentCapacity _asbp_inventory_item) (Variables|/Game/GameProject/Blueprints/Inventory/Items/BP_BaseItemObject.BP_BaseItemObject_C|GetItemSize (.item Item)))))

(fn SpawnRemovedItems
  (params (Item :type Item%20Structure%20Structure))
  (bind _returnvalue (Components|GetOwner))
  (bind _name (Variables|/Game/GameProject/Blueprints/Inventory/Items/BP_BaseItemObject.BP_BaseItemObject_C|GetName (.item Item)))
  (bind _staticmesh (Variables|/Game/GameProject/Blueprints/Inventory/Items/BP_BaseItemObject.BP_BaseItemObject_C|GetStaticMesh (.item Item)))
  (bind _skeletalmesh (Variables|/Game/GameProject/Blueprints/Inventory/Items/BP_BaseItemObject.BP_BaseItemObject_C|GetSkeletalMesh (.item Item)))
  (bind _description (Variables|/Game/GameProject/Blueprints/Inventory/Items/BP_BaseItemObject.BP_BaseItemObject_C|GetDescription (.item Item)))
  (bind _icon (Variables|/Game/GameProject/Blueprints/Inventory/Items/BP_BaseItemObject.BP_BaseItemObject_C|GetIcon (.item Item)))
  (bind _itemsize (Variables|/Game/GameProject/Blueprints/Inventory/Items/BP_BaseItemObject.BP_BaseItemObject_C|GetItemSize (.item Item)))
  (bind _maxstacksize (Variables|/Game/GameProject/Blueprints/Inventory/Items/BP_BaseItemObject.BP_BaseItemObject_C|GetMaxStackSize (.item Item)))
  (bind _equipmenttype (Variables|/Game/GameProject/Blueprints/Inventory/Items/BP_BaseItemObject.BP_BaseItemObject_C|GetEquipmentType (.item Item)))
  (bind _returnvalue_2 (Transformation|GetActorTransform _returnvalue))
  (for _index (range 1 (.amount Item))
    (switch Utilities|FlowControl|Switch|SwitchonEquipmentType (Variables|/Game/GameProject/Blueprints/Inventory/Items/BP_BaseItemObject.BP_BaseItemObject_C|GetEquipmentType (.item Item))
      (:NewEnumerator6
        (bind _returnvalue_3 (Game|SpawnActorfromClass (Variables|/Game/GameProject/Blueprints/Inventory/Items/BP_BaseItemObject.BP_BaseItemObject_C|GetItemClass (.item Item)) _returnvalue_2 "Undefined" 0 (Utilities|Struct|MakeBaseData _name _description _icon _equipmenttype _itemsize) 1 _maxstacksize _skeletalmesh _staticmesh 0 :!label _label))
        (LocalVariables|SetSpawned _returnvalue_3)
        (Physics|SetSimulatePhysics (Variables|/Game/GameProject/Blueprints/Inventory/Items/BP_MasterItem.BP_MasterItem_C|GetStaticMesh _returnvalue_3) true))
      (:NewEnumerator1
        (bind _asbp_inventory_item (Utilities|Casting|CastToBP_InventoryItem (.item Item) :!label _label_2))
        (bind _returnvalue_4 (Game|SpawnActorfromClass (Variables|/Game/GameProject/Blueprints/Inventory/Items/BP_InventoryItem.BP_InventoryItem_C|GetEquipmentClass _asbp_inventory_item) _returnvalue_2 "Undefined" 0 (Utilities|Struct|MakeInventoryItemStructure (Variables|/Game/GameProject/Blueprints/Inventory/Items/BP_InventoryItem.BP_InventoryItem_C|GetInventory _asbp_inventory_item) (Variables|/Game/GameProject/Blueprints/Inventory/Items/BP_InventoryItem.BP_InventoryItem_C|GetMaxCapacity _asbp_inventory_item) (Variables|/Game/GameProject/Blueprints/Inventory/Items/BP_InventoryItem.BP_InventoryItem_C|GetCurrentCapacity _asbp_inventory_item) (Variables|/Game/GameProject/Blueprints/Inventory/Items/BP_InventoryItem.BP_InventoryItem_C|GetInventorySize _asbp_inventory_item)) (Variables|/Game/GameProject/Blueprints/Inventory/Items/BP_InventoryItem.BP_InventoryItem_C|GetEquipmentClass _asbp_inventory_item) (Utilities|Struct|MakeBaseData _name _description _icon _equipmenttype _itemsize) 1 _maxstacksize _skeletalmesh _staticmesh 0))
        (LocalVariables|SetSpawned _returnvalue_4)
        (Physics|SetSimulatePhysics (Variables|/Game/GameProject/Blueprints/Inventory/Items/BP_MasterItem.BP_MasterItem_C|GetStaticMesh _returnvalue_4) true))
      (:NewEnumerator0
        (goto _label_2))
      (:NewEnumerator2
        (goto _label_2))
      (:NewEnumerator3
        (goto _label))
      (:NewEnumerator4
        (goto _label))
      (:NewEnumerator5
        (goto _label))
      (:NewEnumerator7
        (goto _label))
      (:NewEnumerator9
        (goto _label))
      (:NewEnumerator8
        (goto _label))
      (:NewEnumerator10
        (goto _label))
      (:NewEnumerator14
        (goto _label))
      (:NewEnumerator18
        (goto _label))
      (:NewEnumerator19
        (goto _label)))
    (ConstructWidgets|RefreshInventory)
    (ConstructWidgets|TraceGround)
    (return (LocalVariables|GetSpawned)))
  (ConstructWidgets|RefreshInventory))

(fn AddItemstotheGround
  (params (Item :type Item%20Structure%20Structure%20%28by%20ref%29) (Actor :type Actor%20Object%20Reference))
  (Utilities|Array|Add (Variables|Default|GetGroundItems) (Utilities|Struct|MakeGroundItem Item Actor)))

(fn RemovefromGround
  (params (ItemIndex :type Integer))
  (bind _grounditems (Variables|Default|GetGroundItems))
  (LocalVariables|SetTempActor (.actorref (Utilities|Array|Get(acopy) _grounditems ItemIndex)))
  (Utilities|Array|RemoveIndex _grounditems ItemIndex)
  (Actor|DestroyActor (LocalVariables|GetTempActor))
  (return))

(fn TraceGround
  (bind _returnvalue (Components|GetOwner))
  (bind _returnvalue_2 (Transformation|GetActorLocation _returnvalue))
  (bind _returnvalue_3 (- (.z _returnvalue_2) 6e+01))
  (bind _returnvalue_4 (Math|Vector|MakeVector (.x _returnvalue_2) (.y _returnvalue_2) _returnvalue_3))
  (Utilities|Array|Clear (Variables|Default|GetGroundItems))
  (bind _outhits (Collision|MultiSphereTraceByChannel _returnvalue_4 _returnvalue_4 6e+02 "TraceTypeQuery3" false 0 "None"))
  (bind _array_element (Utilities|Array|ForEachLoopwithBreak _outhits)
    (:LoopBody
      (bind _asthird_person_character (Utilities|Casting|CastToThirdPersonCharacter (Components|GetOwner)))
      (Class|BIInteraction|GroundInteraction(Message) (.HitActor (Collision|BreakHitResult _array_element)) _asthird_person_character))
    (:Completed
      (ConstructWidgets|RefreshInventory))))

(fn SwapGroundandSlot
  (params (EquipmentSlots :type Array%20of%20Item%20Structure%20Structures) (SlotItem :type Item%20Structure%20Structure%20%28by%20ref%29) (GroundItem :type Item%20Structure%20Structure%20%28by%20ref%29) (Index :type Integer))
  (Utilities|Array|SetArrayElem EquipmentSlots (Math|Conversions|ToInteger(Byte) (Variables|/Game/GameProject/Blueprints/Inventory/Items/BP_BaseItemObject.BP_BaseItemObject_C|GetEquipmentType (.Item (Utilities|Struct|BreakItemStructure SlotItem)))) GroundItem)
  (Add/Remove|RemovefromGround Index)
  (Add/Remove|SpawnRemovedItems SlotItem)
  (ConstructWidgets|RefreshInventory))

(fn AddItemtoContainer
  (params (Item :type Item%20Structure%20Structure))
  (bind _containeritems (Variables|Default|GetContainerItems))
  (bind (_array_element _array_index) (Utilities|Array|ForEachLoopwithBreak _containeritems :!label _label)
    (:LoopBody
      (Utilities|IsValid? _array_element
        (:IsValid
          (LocalVariables|SetLocalIndex _array_index)
          (LocalVariables|SetLocalSlot _array_element)
          (if (and (Checks|SameItems? (LocalVariables|GetLocalSlot) Item) (Checks|IsStackAvaliable? (LocalVariables|GetLocalSlot)))
            (Utilities|Array|SetArrayElem _containeritems (LocalVariables|GetLocalIndex) (Utilities|Struct|MakeItemStructure (.item (LocalVariables|GetLocalSlot)) (+ (.amount (LocalVariables|GetLocalSlot)) 1)))
            (LocalVariables|SetSuccess true)
            (goto _label Break)
            (else
              (LocalVariables|SetSuccess false))))
        (:IsNotValid
          (LocalVariables|SetEmptySlotIndex _array_index)
          (LocalVariables|SetFoundEmptySlot true))))
    (:Completed
      (if (LocalVariables|GetSuccess)
        _
        (elif (LocalVariables|GetFoundEmptySlot)
          (Utilities|Array|SetArrayElem _containeritems (LocalVariables|GetEmptySlotIndex) (Utilities|Struct|MakeItemStructure (.item Item) 1))
          (LocalVariables|SetSuccess true)
          (else
            (return false Item))))
      (ConstructWidgets|RefreshInventory)
      (return true (Utilities|Struct|MakeItemStructure (.item Item) (- (.amount Item) 1))))))

(fn Initialize
  (params (ContainerSize :type Integer))
  (for _index (range 0 (- ContainerSize 1))
    (bind _returnvalue (Game|ConstructObjectfromClass self "/Game/GameProject/Blueprints/Inventory/Items/BP_BaseItemObject.BP_BaseItemObject_C" "" "" 0 0 "NewEnumerator6" 1 1 0 0))
    (Utilities|Array|Add (Variables|Default|GetContainerItems) (Utilities|Struct|MakeItemStructure _returnvalue 0))))

(fn SwapContainerandSlot
  (params (EquipmentSlots :type Array%20of%20Item%20Structure%20Structures) (Index :type Integer) (SlotItem :type Item%20Structure%20Structure%20%28by%20ref%29) (ContainerItem :type Item%20Structure%20Structure%20%28by%20ref%29))
  (LocalVariables|SetTempItem SlotItem)
  (Utilities|Array|SetArrayElem EquipmentSlots (Math|Conversions|ToInteger(Byte) (Variables|/Game/GameProject/Blueprints/Inventory/Items/BP_BaseItemObject.BP_BaseItemObject_C|GetEquipmentType (.Item (Utilities|Struct|BreakItemStructure SlotItem)))) ContainerItem)
  (Utilities|Array|SetArrayElem (Variables|Default|GetContainerItems) Index (LocalVariables|GetTempItem)))

(fn SwapSlotandContainer
  (params (EquipmentSlots :type Array%20of%20Item%20Structure%20Structures) (Index :type Integer) (ContainerItem :type Item%20Structure%20Structure%20%28by%20ref%29) (SlotItem :type Item%20Structure%20Structure%20%28by%20ref%29))
  (LocalVariables|SetTempItem ContainerItem)
  (Utilities|Array|SetArrayElem (Variables|Default|GetContainerItems) Index SlotItem)
  (Utilities|Array|SetArrayElem EquipmentSlots (Math|Conversions|ToInteger(Byte) (Variables|/Game/GameProject/Blueprints/Inventory/Items/BP_BaseItemObject.BP_BaseItemObject_C|GetEquipmentType (.Item (Utilities|Struct|BreakItemStructure SlotItem)))) (LocalVariables|GetTempItem)))

(fn RemoveAmountfromContainer
  (params (ItemIndex :type Integer) (AmountToRemove :type Integer))
  (bind _containeritems (Variables|Default|GetContainerItems))
  (LocalVariables|SetInventoryItem (Utilities|Array|Get(acopy) _containeritems ItemIndex))
  (LocalVariables|SetAmountInInventory (- (.amount (LocalVariables|GetInventoryItem)) AmountToRemove))
  (if (<= (LocalVariables|GetAmountInInventory) 0)
    (Utilities|Array|RemoveIndex _containeritems ItemIndex)
    (return (LocalVariables|GetInventoryItem))
    (else
      (Utilities|Array|SetArrayElem _containeritems ItemIndex (Utilities|Struct|MakeItemStructure (.item (LocalVariables|GetInventoryItem)) (LocalVariables|GetAmountInInventory)))
      (return (Utilities|Struct|MakeItemStructure (.item (LocalVariables|GetInventoryItem)) AmountToRemove)))))