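; BP_Container is an interactable loot container that fills its inventory component with random items when play begins.
; On BeginPlay it repeatedly picks food, an M4a1 weapon or water at random, constructs a BP_BaseItemObject with hardcoded data and adds it to BPCInventory.
; Interact calls ToggleInventory on the interacting character's inventory, passing itself as the container to open.
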(event EventInteract
  (params (Char :type Third%20Person%20Character%20Object%20Reference))
  (Default|ToggleInventory (Variables|/Game/GameProject/Blueprints/ThirdPersonCharacter.ThirdPersonCharacter_C|GetInventory Char) "NewEnumerator0" self))

(event EventBeginPlay
  (for _index (range 0 15)
    (switch int (Math|Random|RandomIntegerinRange 0 2)
      (:0
        (bind _returnvalue (Game|ConstructObjectfromClass self "/Game/GameProject/Blueprints/Inventory/Items/BP_BaseItemObject.BP_BaseItemObject_C" "food" "SmthToEat" "/Game/GameProject/Textures/Icons/ItemsIcons/Food/1303544.1303544" "/Game/GameProject/Blueprints/Inventory/Items/Useable/BP_Food.BP_Food_C" "NewEnumerator6" 1 4 0 0))
        (Default|AddItemtoContainer (Variables|Default|GetBPC_Inventory) (Utilities|Struct|MakeItemStructure _returnvalue 1)))
      (:1
        (bind _returnvalue_2 (Game|ConstructObjectfromClass self "/Game/GameProject/Blueprints/Inventory/Items/BP_BaseItemObject.BP_BaseItemObject_C" "M4a1" "SmthToShoot" "/Game/GameProject/Textures/Icons/ItemsIcons/Weapon/m4icon.m4icon" "/Game/GameProject/Blueprints/Inventory/Items/Equipables/Wpn/BP_AK.BP_AK_C" "NewEnumerator3" 1 1 0 0))
        (Default|AddItemtoContainer (Variables|Default|GetBPC_Inventory) (Utilities|Struct|MakeItemStructure _returnvalue_2 1)))
      (:2
        (bind _returnvalue_3 (Game|ConstructObjectfromClass self "/Game/GameProject/Blueprints/Inventory/Items/BP_BaseItemObject.BP_BaseItemObject_C" "Water" "SmthToIt" "/Game/GameProject/Textures/Icons/ItemsIcons/Food/824239.824239" "/Game/GameProject/Blueprints/Inventory/Items/Useable/BP_Water.BP_Water_C" "NewEnumerator6" 1 2 0 0))
        (Default|AddItemtoContainer (Variables|Default|GetBPC_Inventory) (Utilities|Struct|MakeItemStructure _returnvalue_3 1))))))

(fn ConstructionScript)